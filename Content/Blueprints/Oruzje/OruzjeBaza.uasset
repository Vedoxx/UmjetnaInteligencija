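; Base weapon Blueprint that handles firing at a fixed cyclic rate.
; OnFireRequested passes a DoOnce gate to fire a round, then a timer calls Ready, which broadcasts OnWeaponFired and resets the gate.
; Each round spawns a bullet at MuzzlePosition, plays a fire sound and runs a debug-drawn line trace.
; The trace result goes unused, as the point damage and AI damage-sense reporting nodes are disconnected.
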(event `OnFireRequested`
  (`/Engine/EditorBlueprintResources/StandardMacros.DoOnce` false :!label _label
    (:`Completed`
      (`self.FireRound`)
      (`KismetSystemLibrary.K2_SetTimer` null "Ready" (`self.CyclicRate`)))))

(event `Ready`
  (`self.OnWeaponFired`)
  (goto _label :!via `Reset`))

(event `FireRound`
  (bind _returnvalue (`SceneComponent.K2_GetComponentLocation` (`self.MuzzlePosition`)))
  (`|SpawnActorFromClass` (`self.BulletClass`) (`SceneComponent.K2_GetComponentToWorld` (`self.MuzzlePosition`)) "AlwaysSpawn" "OverrideRootScale" null null)
  (`GameplayStatics.PlaySoundAtLocation` "/Game/FirstPerson/Audio/FirstPersonTemplateWeaponFire02.FirstPersonTemplateWeaponFire02" _returnvalue (struct) 1.0 1.0 0.0 null null null)
  (bind (_outhit _returnvalue_2) (`KismetSystemLibrary.LineTraceSingle` :`Start` _returnvalue :`End` (+ _returnvalue (* (`SceneComponent.GetForwardVector` (`self.MuzzlePosition`)) (`self.WeaponRange`))) :`TraceChannel` "TraceTypeQuery1" :`DrawDebugType` "ForDuration"))
  (if _returnvalue_2
    _))

(event `self.MuzzlePosition.PhysicsVolumeChangedDelegate`
  (params (NewVolume :type "PhysicsVolume Object Reference")))

(fn `UserConstructionScript`)